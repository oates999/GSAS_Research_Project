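; BP_Note is an actor that displays one sheet-music element, a note, rest or chord, from its Note data.
; BeginPlay derives accidental-free names, picks meshes for type, accidental and articulation, and parses beam tags.
; Chords sort pitches by octave and letter, then build mesh components per pitch.
; Other functions spawn attached ledger lines and stems (BP_Beam), flip notes by negative scaling, and interpolate stem ends along continuing beams.
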(event EventBeginPlay
  (Utilities|FlowControl|Sequence
    (:then_0
      (CallFunction|SetSimpleName))
    (:then_1
      (CallFunction|UpdateMeshes))
    (:then_2
      (if (Utilities|Enum|NotEqual(Enum) (.beams (Utilities|Struct|BreakNote (Variables|Default|Getnote))) "none")
        (for _array_element (Utilities|GetBeamArray (Variables|Default|Getnote))
          (Utilities|Array|Add (Variables|Default|Getbeams) (.RightS (Utilities|String|Split _array_element "[b]"))))
        (else
          (Utilities|Array|Add (Variables|Default|Getbeams) "none"))))))

(fn ConstructionScript
  (if (.is_rest (Utilities|Struct|BreakNote (Variables|Default|Getnote)))
    (Rendering|SetVisibility (Variables|Default|Getaccidental_mesh) false true)
    (Rendering|SetVisibility (Variables|Default|Getarticulation_mesh) false true)))

(fn UpdateMeshes
  (bind _note_meshes (Variables|Default|Getnote_meshes))
  (bind _note (Variables|Default|Getnote))
  (bind (_offset _is_note _is_chord _is_rest _name _pitches _chord_symbol _chord_type _type _quarter_length _dots _articulations) (Utilities|Struct|BreakNote _note))
  (bind (_value _returnvalue) (Utilities|Map|Find _note_meshes _type))
  (bind _returnvalue_2 (Utilities|String|GetCharacterArrayfromString _name))
  (Utilities|FlowControl|Sequence
    (:then_0
      ;[1 1 1] Set Primary Mesh
      (if _is_note
        (if _returnvalue
          (Components|StaticMesh|SetStaticMesh (Variables|Default|Getnote_primary_mesh) _value)
          (else
            (Development|PrintString "ERROR: key not found")))
        (elif _is_rest
          (Components|StaticMesh|SetStaticMesh (Variables|Default|Getnote_primary_mesh) (.Value (Utilities|Map|Find (Variables|Default|Getrest_meshes) _type)))
          (elif _is_chord
            (CallFunction|UpdateChordMeshes)))))
    (:then_1
      ;[1 1 1] Set Accidental Mesh
      (if _is_note
        (if (!= (Utilities|Array|FindItem _returnvalue_2 "#") -1)
          (Components|StaticMesh|SetStaticMesh (Variables|Default|Getaccidental_mesh) "/Game/Assets/StaticMeshes/notation_sharp.notation_sharp")
          (elif (!= (Utilities|Array|FindItem _returnvalue_2 "-") -1)
            (Components|StaticMesh|SetStaticMesh (Variables|Default|Getaccidental_mesh) "/Game/Assets/StaticMeshes/notation_flat.notation_flat")
            (else
              (Rendering|SetVisibility (Variables|Default|Getaccidental_mesh) false true))))))
    (:then_2
      ;[1 1 1] Set Dot Mesh
      (if (not (> _dots 0))
        (Rendering|SetVisibility (Variables|Default|Getdot_mesh) false true)))
    (:then_3
      ;[1 1 1] Set Articulation Mesh
      (if (Utilities|Enum|NotEqual(Enum) _articulations "noArt")
        (if true
          (Components|StaticMesh|SetStaticMesh (Variables|Default|Getarticulation_mesh) (.Value (Utilities|Map|Find (Variables|Default|Getarticulation_meshes) _articulations))))
        (else
          (Rendering|SetVisibility (Variables|Default|Getarticulation_mesh) false true))))
    (:then_4
      ;[1 1 1] Set Chord Symbol
      (if _is_chord
        (Rendering|Components|TextRender|SetText (Variables|Default|Getchord_symbol) (Utilities|Text|ToText(String) _chord_symbol))
        (if (Utilities|Enum|Equal(Enum) _type "zero")
          (Development|SetHiddeninGame (Variables|Default|Getnote_primary_mesh) true true)
          (Development|SetHiddeninGame (Variables|Default|Getdot_mesh) true true)
          (Development|SetHiddeninGame (Variables|Default|Getarticulation_mesh) true true)
          (Development|SetHiddeninGame (Variables|Default|Getaccidental_mesh) true true))
        (else
          (Development|SetHiddeninGame (Variables|Default|Getchord_symbol) true false))))))

(fn AddLedgerLines
  (bind _self self)
  (bind _required_ledgers (Variables|Default|Getrequired_ledgers))
  (bind _returnvalue (Transformation|GetActorTransform _self))
  (if (> (Utilities|Array|Length _required_ledgers) 0)
    (Utilities|Array|Clear (Variables|Default|Getledger_lines))
    (for _array_element _required_ledgers
      (bind _returnvalue_2 (Game|SpawnActorfromClass "/Game/Blueprints/BP_LedgerLine.BP_LedgerLine_C" (Math|Transform|MakeTransform (Math|Vector|MakeVector (.x (.location _returnvalue)) (.y (.location _returnvalue)) (.z _array_element)) (.rotation _returnvalue) (.scale _returnvalue)) "Undefined" 0 0))
      (Utilities|Array|Add (Variables|Default|Getledger_lines) _returnvalue_2)
      (Transformation|AttachActorToActor _returnvalue_2 self "None" "KeepWorld" "KeepWorld" "KeepWorld" false))))

(fn SwaptoAltMeshifNeeded
  (bind _note (Variables|Default|Getnote))
  (bind _alt_meshes (Variables|Default|Getalt_meshes))
  (bind _type (Utilities|Struct|BreakNote _note))
  (bind (_value _returnvalue) (Utilities|Map|Find _alt_meshes _type))
  (if _returnvalue
    (Components|StaticMesh|SetStaticMesh (Variables|Default|Getnote_primary_mesh) _value)))

(fn UpdateBeamMeshes
  (params (previous_flipped :type Boolean))
  (bind _beam_attach_point (Variables|Default|Getbeam_attach_point))
  (bind _bulb_attach_point (Variables|Default|Getbulb_attach_point))
  (bind _note_primary_mesh (Variables|Default|Getnote_primary_mesh))
  (bind _note_primary_mesh_2 (Variables|Default|Getnote_primary_mesh))
  (bind _beam_attach_point_2 (Variables|Default|Getbeam_attach_point))
  (bind _bulb_attach_point_2 (Variables|Default|Getbulb_attach_point))
  (bind _relativescale3d (Variables|/Script/Engine.SceneComponent|GetRelativeScale3D _note_primary_mesh))
  (bind _relativescale3d_2 (Variables|/Script/Engine.SceneComponent|GetRelativeScale3D _note_primary_mesh_2))
  (if (not (.is_chord (Utilities|Struct|BreakNote (Variables|Default|Getnote))))
    (Utilities|FlowControl|Sequence
      (:then_0
        ;[1 1 1] Note
        ;;[1 1 1] Note Flipping (if needed)
        (if (Math|Boolean|NotEqual(Boolean) previous_flipped (Variables|Default|Getflipped))
          (Transformation|SetRelativeScale3D _note_primary_mesh_2 (Math|Vector|MakeVector (* -1 (.x _relativescale3d_2)) (.y _relativescale3d_2) (* -1 (.z _relativescale3d_2))))
          (Variables|Default|Setflipped previous_flipped)))
      (:then_1
        ;;[1 1 1] Vertical Beam Spawning
        (Components|StaticMesh|SetStaticMesh (Variables|Default|Getnote_primary_mesh) "/Game/Assets/StaticMeshes/note_bulbOnly.note_bulbOnly")
        (if (> (.z (Transformation|GetWorldLocation _beam_attach_point)) (.z (Transformation|GetWorldLocation _bulb_attach_point)))
          (bind _returnvalue (Game|SpawnActorfromClass "/Game/Blueprints/BP_Beam.BP_Beam_C" (Transformation|GetWorldTransform _bulb_attach_point) "Undefined" 0 (Transformation|GetWorldLocation _beam_attach_point) 0))
          (Transformation|AttachActorToActor _returnvalue self "None" "KeepWorld" "KeepWorld" "KeepWorld" false)
          (else
            (bind _returnvalue_2 (Game|SpawnActorfromClass "/Game/Blueprints/BP_Beam.BP_Beam_C" (Transformation|GetWorldTransform _beam_attach_point) "Undefined" 0 (Transformation|GetWorldLocation _bulb_attach_point) 0))
            (Transformation|AttachActorToActor _returnvalue_2 self "None" "KeepWorld" "KeepWorld" "KeepWorld" false)))))
    (else
      (Utilities|FlowControl|Sequence
        (:then_0
          ;[1 1 1] Chord
          ;;[1 1 1] Note Flipping (if needed)
          (if (Math|Boolean|NotEqual(Boolean) previous_flipped (Variables|Default|Getflipped))
            (Transformation|SetRelativeScale3D _note_primary_mesh (Math|Vector|MakeVector (* -1 (.x _relativescale3d)) (.y _relativescale3d) (* -1 (.z _relativescale3d))))
            (Variables|Default|Setflipped previous_flipped)
            (for _array_element (Variables|Default|Getpitch_mesh_components)
              (for _array_element_2 (Components|GetChildrenComponents _array_element false)
                (bind _asstatic_mesh_component (Utilities|Casting|CastToStaticMeshComponent _array_element_2))
                (Transformation|SetRelativeScale3D _asstatic_mesh_component (Math|Vector|MakeVector (* -1 (.x (Variables|/Script/Engine.SceneComponent|GetRelativeScale3D _asstatic_mesh_component))) (.y (Variables|/Script/Engine.SceneComponent|GetRelativeScale3D _asstatic_mesh_component)) (* -1 (.z (Variables|/Script/Engine.SceneComponent|GetRelativeScale3D _asstatic_mesh_component)))))))))
        (:then_1
          ;;[1 1 1] Vertical Beam Spawning
          (Components|StaticMesh|SetStaticMesh (Variables|Default|Getnote_primary_mesh) "/Game/Assets/StaticMeshes/note_bulbOnly.note_bulbOnly")
          (if (> (.z (Transformation|GetWorldLocation _beam_attach_point_2)) (.z (Transformation|GetWorldLocation _bulb_attach_point_2)))
            (bind _returnvalue_3 (Game|SpawnActorfromClass "/Game/Blueprints/BP_Beam.BP_Beam_C" (Transformation|GetWorldTransform _bulb_attach_point_2) "Undefined" 0 (Transformation|GetWorldLocation _beam_attach_point_2) 0))
            (Transformation|AttachActorToActor _returnvalue_3 self "None" "KeepWorld" "KeepWorld" "KeepWorld" false)
            (else
              (bind _returnvalue_4 (Game|SpawnActorfromClass "/Game/Blueprints/BP_Beam.BP_Beam_C" (Transformation|GetWorldTransform _beam_attach_point_2) "Undefined" 0 (Transformation|GetWorldLocation _bulb_attach_point_2) 0))
              (Transformation|AttachActorToActor _returnvalue_4 self "None" "KeepWorld" "KeepWorld" "KeepWorld" false))))))))

(fn UpdateContinueBeamMeshes
  (params (beam_start_point :type Vector) (beam_end_point :type Vector) (previous_flipped :type Boolean))
  (bind _x (Math|Vector|BreakVector beam_start_point))
  (bind _note_primary_mesh (Variables|Default|Getnote_primary_mesh))
  (bind _beam_attach_point (Variables|Default|Getbeam_attach_point))
  (bind _bulb_attach_point (Variables|Default|Getbulb_attach_point))
  (bind _relativescale3d (Variables|/Script/Engine.SceneComponent|GetRelativeScale3D _note_primary_mesh))
  (Utilities|FlowControl|Sequence
    (:then_0
      ;[1 1 1] Note Flipping (if needed)
      (if (Math|Boolean|NotEqual(Boolean) previous_flipped (Variables|Default|Getflipped))
        (Transformation|SetRelativeScale3D _note_primary_mesh (Math|Vector|MakeVector (* -1 (.x _relativescale3d)) (.y _relativescale3d) (* -1 (.z _relativescale3d))))
        (Variables|Default|Setflipped previous_flipped)))
    (:then_1
      (Transformation|SetWorldLocation (Variables|Default|Getbeam_attach_point) (+ beam_start_point (* (- beam_end_point beam_start_point) (/ (- (.X (Math|Vector|BreakVector (Transformation|GetWorldLocation (Variables|Default|Getbulb_attach_point)))) _x) (- (.X (Math|Vector|BreakVector beam_end_point)) _x)))) false true)
      ;[1 1 1] Vertical Beam Spawning
      (Components|StaticMesh|SetStaticMesh (Variables|Default|Getnote_primary_mesh) "/Game/Assets/StaticMeshes/note_bulbOnly.note_bulbOnly")
      (if (> (.z (Transformation|GetWorldLocation _beam_attach_point)) (.z (Transformation|GetWorldLocation _bulb_attach_point)))
        (bind _returnvalue (Game|SpawnActorfromClass "/Game/Blueprints/BP_Beam.BP_Beam_C" (Transformation|GetWorldTransform _bulb_attach_point) "Undefined" 0 (Transformation|GetWorldLocation _beam_attach_point) 0))
        (Transformation|AttachActorToActor _returnvalue self "None" "KeepWorld" "KeepWorld" "KeepWorld" false)
        (else
          (bind _returnvalue_2 (Game|SpawnActorfromClass "/Game/Blueprints/BP_Beam.BP_Beam_C" (Transformation|GetWorldTransform _beam_attach_point) "Undefined" 0 (Transformation|GetWorldLocation _bulb_attach_point) 0))
          (Transformation|AttachActorToActor _returnvalue_2 self "None" "KeepWorld" "KeepWorld" "KeepWorld" false))))))

(fn SetSimpleName
  (bind _note (Variables|Default|Getnote))
  (bind (_offset _is_note _is_chord _is_rest _name) (Utilities|Struct|BreakNote _note))
  (bind _returnvalue (Utilities|String|FindSubstring _name "#"))
  (bind _returnvalue_2 (Utilities|String|FindSubstring _name "-"))
  (bind (_lefts _rights) (Utilities|String|Split _name "#"))
  (bind (_lefts_2 _rights_2) (Utilities|String|Split _name "-"))
  (bind _returnvalue_3 (== _returnvalue -1))
  (bind _returnvalue_4 (== _returnvalue_2 -1))
  (if _is_note
    ;[1 1 1] Note
    (if (and _returnvalue_3 _returnvalue_4)
      (Variables|Default|Setsimple_name _name)
      (elif (not _returnvalue_3)
        (Variables|Default|Setsimple_name (Utilities|String|Append _lefts _rights))
        (elif (not _returnvalue_4)
          (Variables|Default|Setsimple_name (Utilities|String|Append _lefts_2 _rights_2)))))
    (elif _is_rest
      ;[1 1 1] Rest
      (Variables|Default|Setsimple_name "REST")
      (elif _is_chord
        ;[1 1 1] Chord
        (bind _pitches_out (CallFunction|SortPitchArray (Utilities|GetPitchArray (Variables|Default|Getnote))))
        (bind _output_get (Variables|Default|Setpitches _pitches_out))
        (CallFunction|SetSimplePitches)
        (if (and (== (Utilities|String|FindSubstring (Utilities|Array|Get(acopy) _output_get) "#") -1) (== (Utilities|String|FindSubstring (Utilities|Array|Get(acopy) _output_get) "-") -1))
          (Variables|Default|Setsimple_name (Utilities|Array|Get(acopy) _output_get))
          (elif (not (== (Utilities|String|FindSubstring (Utilities|Array|Get(acopy) _output_get) "#") -1))
            (Variables|Default|Setsimple_name (Utilities|String|Append (.LeftS (Utilities|String|Split (Utilities|Array|Get(acopy) _output_get) "#")) (.RightS (Utilities|String|Split (Utilities|Array|Get(acopy) _output_get) "#"))))
            (elif (not (== (Utilities|String|FindSubstring (Utilities|Array|Get(acopy) _output_get) "-") -1))
              (Variables|Default|Setsimple_name (Utilities|String|Append (.LeftS (Utilities|String|Split (Utilities|Array|Get(acopy) _output_get) "-")) (.RightS (Utilities|String|Split (Utilities|Array|Get(acopy) _output_get) "-")))))))))))

(fn SortPitchArray
  (params (pitches_in :type Array%20of%20Strings))
  (while (> (Utilities|Array|Length pitches_in) 0)
    (LocalVariables|Setcurrent_lowest 0)
    (for (_array_element _array_index) pitches_in
      ;[1 1 1] Octave Compare --> Note Compare
      (if (< (Math|Conversions|ToInteger(Byte) (Utilities|Array|Get(acopy) (Utilities|String|GetCharacterArrayfromString _array_element) (- (Utilities|Array|Length (Utilities|String|GetCharacterArrayfromString _array_element)) 1))) (Math|Conversions|ToInteger(Byte) (Utilities|Array|Get(acopy) (Utilities|String|GetCharacterArrayfromString (Utilities|Array|Get(acopy) pitches_in (LocalVariables|Getcurrent_lowest))) (- (Utilities|Array|Length (Utilities|String|GetCharacterArrayfromString (Utilities|Array|Get(acopy) pitches_in (LocalVariables|Getcurrent_lowest)))) 1))))
        (LocalVariables|Setcurrent_lowest _array_index)
        (elif (Math|Boolean|ANDBoolean (== (Math|Conversions|ToInteger(Byte) (Utilities|Array|Get(acopy) (Utilities|String|GetCharacterArrayfromString _array_element) (- (Utilities|Array|Length (Utilities|String|GetCharacterArrayfromString _array_element)) 1))) (Math|Conversions|ToInteger(Byte) (Utilities|Array|Get(acopy) (Utilities|String|GetCharacterArrayfromString (Utilities|Array|Get(acopy) pitches_in (LocalVariables|Getcurrent_lowest))) (- (Utilities|Array|Length (Utilities|String|GetCharacterArrayfromString (Utilities|Array|Get(acopy) pitches_in (LocalVariables|Getcurrent_lowest)))) 1)))) (< (.Value (Utilities|Map|Find (Variables|Default|Getnote_numbers) (Utilities|Array|Get(acopy) (Utilities|String|GetCharacterArrayfromString _array_element)))) (.Value (Utilities|Map|Find (Variables|Default|Getnote_numbers) (Utilities|Array|Get(acopy) (Utilities|String|GetCharacterArrayfromString (Utilities|Array|Get(acopy) pitches_in (LocalVariables|Getcurrent_lowest))))))) (.ReturnValue (Utilities|Map|Find (Variables|Default|Getnote_numbers) (Utilities|Array|Get(acopy) (Utilities|String|GetCharacterArrayfromString _array_element)))) (.ReturnValue (Utilities|Map|Find (Variables|Default|Getnote_numbers) (Utilities|Array|Get(acopy) (Utilities|String|GetCharacterArrayfromString (Utilities|Array|Get(acopy) pitches_in (LocalVariables|Getcurrent_lowest)))))))
          (LocalVariables|Setcurrent_lowest _array_index))))
    ;[1 1 1] Add/Remove Lowest Note
    (Utilities|Array|Add (LocalVariables|Getsorted_pitches) (Utilities|Array|Get(acopy) pitches_in (LocalVariables|Getcurrent_lowest)))
    (Utilities|Array|RemoveIndex pitches_in (LocalVariables|Getcurrent_lowest)))
  ;[1 1 1] Return Sorted Array
  (return (LocalVariables|Getsorted_pitches)))

(fn SetSimplePitches
  (for _array_element (Variables|Default|Getpitches)
    (if (and (== (Utilities|String|FindSubstring _array_element "#") -1) (== (Utilities|String|FindSubstring _array_element "-") -1))
      (Utilities|Array|Add (Variables|Default|Getsimple_pitches) _array_element)
      (elif (not (== (Utilities|String|FindSubstring _array_element "#") -1))
        (Utilities|Array|Add (Variables|Default|Getsimple_pitches) (Utilities|String|Append (.LeftS (Utilities|String|Split _array_element "#")) (.RightS (Utilities|String|Split _array_element "#"))))
        (elif (not (== (Utilities|String|FindSubstring _array_element "-") -1))
          (Utilities|Array|Add (Variables|Default|Getsimple_pitches) (Utilities|String|Append (.LeftS (Utilities|String|Split _array_element "-")) (.RightS (Utilities|String|Split _array_element "-")))))))))

(fn UpdateChordMeshes
  (bind _note (Variables|Default|Getnote))
  (bind _type (Utilities|Struct|BreakNote _note))
  (Rendering|SetVisibility (Variables|Default|Getnote_primary_mesh) false false)
  (Rendering|SetVisibility (Variables|Default|Getdot_mesh) false false)
  (Rendering|SetVisibility (Variables|Default|Getaccidental_mesh) false false)
  (Utilities|FlowControl|Sequence
    (:then_0
      ;[1 1 1] Determine Bulb Mesh
      (if (Utilities|Enum|Equal(Enum) _type "whole")
        (LocalVariables|Setlocal_bulb_mesh "/Game/Assets/StaticMeshes/note_whole.note_whole")
        (elif (Utilities|Enum|Equal(Enum) _type "half")
          (LocalVariables|Setlocal_bulb_mesh "/Game/Assets/StaticMeshes/note_bulbOnly_half.note_bulbOnly_half")
          (else
            (LocalVariables|Setlocal_bulb_mesh "/Game/Assets/StaticMeshes/note_bulbOnly.note_bulbOnly")))))
    (:then_1
      ;[1 1 1] Add Static Mesh Components
      (for _array_element (Variables|Default|Getpitches)
        (bind _returnvalue (AddComponent|AddStaticMeshComponent true (Transformation|GetActorTransform self)))
        (Components|StaticMesh|SetStaticMesh _returnvalue (LocalVariables|Getlocal_bulb_mesh))
        (Transformation|AttachComponentToComponent _returnvalue (Variables|Default|Getnote_primary_mesh) "None" "KeepWorld" "KeepWorld" "KeepWorld" false)
        (Utilities|Array|Add (Variables|Default|Getpitch_mesh_components) _returnvalue)))
    (:then_2
      ;[1 1 1] Accidental Meshes
      (for (_array_element_2 _array_index) (Variables|Default|Getpitches)
        (if (not (== (Utilities|String|FindSubstring _array_element_2 "#") -1))
          (bind _returnvalue_2 (AddComponent|AddStaticMeshComponent true (Transformation|GetWorldTransform (Variables|Default|Getaccidental_mesh))))
          (Transformation|AttachComponentToComponent _returnvalue_2 (Utilities|Array|Get(acopy) (Variables|Default|Getpitch_mesh_components) _array_index) "None" "KeepWorld" "KeepWorld" "KeepWorld" false)
          (elif (not (== (Utilities|String|FindSubstring _array_element_2 "-") -1))
            (bind _returnvalue_3 (AddComponent|AddStaticMeshComponent true (Transformation|GetWorldTransform (Variables|Default|Getaccidental_mesh))))
            (Transformation|AttachComponentToComponent _returnvalue_3 (Utilities|Array|Get(acopy) (Variables|Default|Getpitch_mesh_components) _array_index) "None" "KeepWorld" "KeepWorld" "KeepWorld" false)))))
    (:then_3
      ;[1 1 1] Dot Meshes
      (for (_ _array_index_2) (Variables|Default|Getpitches)
        (if (> (.dots (Utilities|Struct|BreakNote (Variables|Default|Getnote))) 0)
          (bind _returnvalue_4 (AddComponent|AddStaticMeshComponent true (Transformation|GetWorldTransform (Variables|Default|Getdot_mesh))))
          (Transformation|AttachComponentToComponent _returnvalue_4 (Utilities|Array|Get(acopy) (Variables|Default|Getpitch_mesh_components) _array_index_2) "None" "KeepWorld" "KeepWorld" "KeepWorld" false))))))

(fn DrawChordVerticalBeams
  (bind _pitch_mesh_components (Variables|Default|Getpitch_mesh_components))
  (bind _bulb_attach_point (Variables|Default|Getbulb_attach_point))
  (bind _returnvalue (Utilities|Array|Length _pitch_mesh_components))
  (bind _returnvalue_2 (Transformation|GetWorldLocation _bulb_attach_point))
  (bind _returnvalue_3 (- _returnvalue 1))
  (bind _output (Utilities|Array|Get(acopy) _pitch_mesh_components _returnvalue_3))
  (if (Utilities|Enum|NotEqual(Enum) (.type (Utilities|Struct|BreakNote (Variables|Default|Getnote))) "whole")
    (bind _returnvalue_4 (Game|SpawnActorfromClass "/Game/Blueprints/BP_Beam.BP_Beam_C" (Transformation|GetWorldTransform (Utilities|Array|Get(acopy) (Variables|Default|Getpitch_mesh_components))) "Undefined" 0 (+ (- (Transformation|GetWorldLocation (Variables|Default|Getbeam_attach_point)) (Transformation|GetWorldLocation (Variables|Default|Getbulb_attach_point))) (Transformation|GetWorldLocation _output)) 0))
    (Transformation|AttachComponentToComponent _returnvalue_4 _output "None" "KeepWorld" "KeepWorld" "KeepWorld" false)
    (Transformation|SetActorLocation _returnvalue_4 (Math|Vector|MakeVector (.x _returnvalue_2) (.y _returnvalue_2) (.z (Transformation|GetActorLocation _returnvalue_4))) false true)))

(fn GetBeamAttachPoints
  (bind _beam_attach_point (Variables|Default|Getbeam_attach_point))
  (bind _pitch_mesh_components (Variables|Default|Getpitch_mesh_components))
  (bind _bulb_attach_point (Variables|Default|Getbulb_attach_point))
  (bind _beam_second_attach_point (Variables|Default|Getbeam_second_attach_point))
  (bind _pitch_mesh_components_2 (Variables|Default|Getpitch_mesh_components))
  (bind _bulb_attach_point_2 (Variables|Default|Getbulb_attach_point))
  (bind _pitch_mesh_components_3 (Variables|Default|Getpitch_mesh_components))
  (bind _bulb_attach_point_3 (Variables|Default|Getbulb_attach_point))
  (bind _note (Variables|Default|Getnote))
  (bind _beam_third_attach_point (Variables|Default|Getbeam_third_attach_point))
  (bind (_offset _is_note _is_chord) (Utilities|Struct|BreakNote _note))
  (bind _returnvalue (Transformation|GetWorldLocation _bulb_attach_point_3))
  (bind _returnvalue_2 (Transformation|GetWorldTransform _beam_third_attach_point))
  (bind _returnvalue_3 (Transformation|GetWorldLocation _bulb_attach_point))
  (bind _returnvalue_4 (Transformation|GetWorldTransform _beam_attach_point))
  (bind _returnvalue_5 (Transformation|GetWorldLocation _bulb_attach_point_2))
  (bind _returnvalue_6 (Transformation|GetWorldTransform _beam_second_attach_point))
  (bind (_x _y) (Math|Vector|BreakVector _returnvalue))
  (bind (_x_2 _y_2) (Math|Vector|BreakVector _returnvalue_3))
  (bind (_x_3 _y_3) (Math|Vector|BreakVector _returnvalue_5))
  (if _is_note
    (return (Transformation|GetWorldTransform (Variables|Default|Getbeam_attach_point)) (Transformation|GetWorldTransform (Variables|Default|Getbeam_second_attach_point)) (Transformation|GetWorldTransform (Variables|Default|Getbeam_third_attach_point)))
    (elif _is_chord
      (return (Math|Transform|MakeTransform (Math|Vector|MakeVector _x_2 _y_2 (.z (+ (- (Transformation|GetWorldLocation _beam_attach_point) _returnvalue_3) (Transformation|GetWorldLocation (Utilities|Array|Get(acopy) _pitch_mesh_components (- (Utilities|Array|Length _pitch_mesh_components) 1)))))) (.rotation _returnvalue_4) (.scale _returnvalue_4)) (Math|Transform|MakeTransform (Math|Vector|MakeVector _x_3 _y_3 (.z (+ (- (Transformation|GetWorldLocation _beam_second_attach_point) _returnvalue_5) (Transformation|GetWorldLocation (Utilities|Array|Get(acopy) _pitch_mesh_components_2 (- (Utilities|Array|Length _pitch_mesh_components_2) 1)))))) (.rotation _returnvalue_6) (.scale _returnvalue_6)) (Math|Transform|MakeTransform (Math|Vector|MakeVector _x _y (.z (+ (- (Transformation|GetWorldLocation _beam_third_attach_point) _returnvalue) (Transformation|GetWorldLocation (Utilities|Array|Get(acopy) _pitch_mesh_components_3 (- (Utilities|Array|Length _pitch_mesh_components_3) 1)))))) (.rotation _returnvalue_2) (.scale _returnvalue_2))))))

(fn GetChordTieOffset
  (bind _pitch_mesh_components (Variables|Default|Getpitch_mesh_components))
  (return (- (Transformation|GetWorldLocation (Utilities|Array|Get(acopy) _pitch_mesh_components (- (Utilities|Array|Length _pitch_mesh_components) 1))) (Transformation|GetWorldLocation (Utilities|Array|Get(acopy) _pitch_mesh_components)))))