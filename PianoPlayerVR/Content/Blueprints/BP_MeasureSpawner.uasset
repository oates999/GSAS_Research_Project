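; Spawner actor that lays out a 3D grand-staff score from treble and bass measure data.
; On BeginPlay it spawns attached BP_Measure actors with notes, spaces them by the arrow offset, then adds beams, begin/mid/end staff meshes and ties.
; Time signature meshes come from the first measure's string.
; Lookup functions scan the spawner's note arrays for tie and beam stops, allowing cross-measure links and updating continued beam notes.
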(event EventBeginPlay
  (CallFunction|SpawnMeasures)
  (CallFunction|UpdateTimeSignatures (Utilities|Array|Get(acopy) (Variables|Default|Getmeasures_treble))))

(fn ConstructionScript)

(fn SpawnMeasures
  (bind _self self)
  (bind _measures (Variables|Default|Getmeasures))
  (Utilities|FlowControl|Sequence
    (:then_0
      ;[1 1 1] Spawn Measures
      (for (_array_element _array_index) (Variables|Default|Getmeasures_treble)
        (bind _returnvalue (Game|SpawnActorfromClass "/Game/Blueprints/BP_Measure.BP_Measure_C" (Transformation|GetActorTransform _self) "Undefined" 0 (Utilities|Array|Get(acopy) (Variables|Default|Getmeasures_bass) _array_index) _array_element _self 0))
        (Utilities|Array|Add (Variables|Default|Getmeasures) _returnvalue)
        (Transformation|AttachActorToActor _returnvalue self "None" "KeepWorld" "KeepWorld" "KeepWorld" false)
        (Default|SpawnNotes _returnvalue)))
    (:then_1
      ;[1 1 1] Reposition Measures
      (for (_array_element_2 _array_index_2) _measures
        (Transformation|SetActorLocation _array_element_2 (+ (* (- (Transformation|GetWorldLocation (Variables|Default|Getend_arrow)) (Transformation|GetWorldLocation (Variables|Default|Getstart_arrow))) _array_index_2) (Transformation|GetWorldLocation (Variables|Default|Getmeasure_start_location))) false true)
        (Default|AddBeamLines _array_element_2)
        (if (== _array_index_2 0)
          (Default|SetStaffMesh _array_element_2 "begin")
          (elif (== _array_index_2 (- (Utilities|Array|Length _measures) 1))
            (Default|SetStaffMesh _array_element_2 "end")
            (else
              (Default|SetStaffMesh _array_element_2 "mid"))))))
    (:then_2
      ;[1 1 1] Add Tie Lines
      (for _array_element_3 (Variables|Default|Getmeasures)
        (Default|AddTieLines _array_element_3)))))

(fn UpdateTimeSignatures
  (params (measure :type Measure%20Structure))
  (bind _time_signature (Utilities|Struct|BreakMeasure measure))
  (bind _number_meshes (Variables|Default|Getnumber_meshes))
  (bind (_lefts _rights _returnvalue) (Utilities|String|Split _time_signature "/"))
  (bind (_value _returnvalue_2) (Utilities|Map|Find _number_meshes _lefts))
  (bind (_value_2 _returnvalue_3) (Utilities|Map|Find _number_meshes _rights))
  (if (Math|Boolean|ANDBoolean _returnvalue _returnvalue_2 _returnvalue_3)
    (Components|StaticMesh|SetStaticMesh (Variables|Default|Gettreble_upper_mesh) _value)
    (Components|StaticMesh|SetStaticMesh (Variables|Default|Getbass_upper_mesh) _value)
    (Components|StaticMesh|SetStaticMesh (Variables|Default|Gettreble_lower_mesh) _value_2)
    (Components|StaticMesh|SetStaticMesh (Variables|Default|Getbass_lower_mesh) _value_2)))

(fn GetTieEndPoint
  (params (start_note :type BP%20Note%20Object%20Reference) (treble? :type Boolean))
  (bind _notes_bass (Variables|Default|Getnotes_bass))
  (bind _notes_treble (Variables|Default|Getnotes_treble))
  (if treble?
    (bind _index (Utilities|FlowControl|ForLoopwithBreak (+ (Utilities|Array|FindItem _notes_treble start_note) 1) (- (Utilities|Array|Length _notes_treble) 1) :!label _label)
      (:LoopBody
        (if (Utilities|Enum|Equal(Enum) (.ties (Utilities|Struct|BreakNote (Variables|/Game/Blueprints/BP_Note.BP_Note_C|Getnote (Utilities|Array|Get(acopy) _notes_treble _index)))) "stop")
          (LocalVariables|Setlocal_return_note (Utilities|Array|Get(acopy) _notes_treble _index))
          (LocalVariables|Setlocal_valid_return true)
          (goto _label Break)))
      (:Completed
        (return (LocalVariables|Getlocal_return_note) (LocalVariables|Getlocal_valid_return))))
    (else
      (bind _index_2 (Utilities|FlowControl|ForLoopwithBreak (+ (Utilities|Array|FindItem _notes_bass start_note) 1) (- (Utilities|Array|Length _notes_bass) 1) :!label _label_2)
        (:LoopBody
          (if (Utilities|Enum|Equal(Enum) (.ties (Utilities|Struct|BreakNote (Variables|/Game/Blueprints/BP_Note.BP_Note_C|Getnote (Utilities|Array|Get(acopy) _notes_bass _index_2)))) "stop")
            (LocalVariables|Setlocal_return_note (Utilities|Array|Get(acopy) _notes_bass _index_2))
            (LocalVariables|Setlocal_valid_return true)
            (goto _label_2 Break)))
        (:Completed
          (return (LocalVariables|Getlocal_return_note) (LocalVariables|Getlocal_valid_return)))))))

(fn GetBeamEndPoint
  (params (start_note :type BP%20Note%20Object%20Reference) (treble? :type Boolean))
  (bind _notes_bass (Variables|Default|Getnotes_bass))
  (bind _notes_treble (Variables|Default|Getnotes_treble))
  (if treble?
    (bind _index (Utilities|FlowControl|ForLoopwithBreak (+ (Utilities|Array|FindItem _notes_treble start_note) 1) (- (Utilities|Array|Length _notes_treble) 1) :!label _label)
      (:LoopBody
        (if (!= (Utilities|Array|FindItem (Variables|/Game/Blueprints/BP_Note.BP_Note_C|Getbeams (Utilities|Array|Get(acopy) _notes_treble _index)) "stop") -1)
          (LocalVariables|Setlocal_valid_return true)
          (goto _label Break)
          (elif (!= (Utilities|Array|FindItem (Variables|/Game/Blueprints/BP_Note.BP_Note_C|Getbeams (Utilities|Array|Get(acopy) _notes_treble _index)) "continue") -1)
            (Utilities|Array|Add (LocalVariables|Getlocal_continued_notes) (Utilities|Array|Get(acopy) _notes_treble _index)))))
      (:Completed
        (Utilities|FlowControl|Sequence
          (:then_0
            (for _array_element (LocalVariables|Getlocal_continued_notes)
              (Variables|/Game/Blueprints/BP_Note.BP_Note_C|Setcontinued _array_element true)
              (Default|UpdateContinueBeamMeshes _array_element (Transformation|GetWorldLocation (Variables|/Game/Blueprints/BP_Note.BP_Note_C|Getbeam_attach_point start_note)) (Transformation|GetWorldLocation (Variables|/Game/Blueprints/BP_Note.BP_Note_C|Getbeam_attach_point (Utilities|Array|Get(acopy) _notes_treble _index))) (Variables|/Game/Blueprints/BP_Note.BP_Note_C|Getflipped start_note))))
          (:then_1
            (return (Utilities|Array|Get(acopy) _notes_treble _index) (LocalVariables|Getlocal_valid_return))))))
    (else
      (bind _index_2 (Utilities|FlowControl|ForLoopwithBreak (+ (Utilities|Array|FindItem _notes_bass start_note) 1) (- (Utilities|Array|Length _notes_bass) 1) :!label _label_2)
        (:LoopBody
          (if (!= (Utilities|Array|FindItem (Variables|/Game/Blueprints/BP_Note.BP_Note_C|Getbeams (Utilities|Array|Get(acopy) _notes_bass _index_2)) "stop") -1)
            (LocalVariables|Setlocal_valid_return true)
            (goto _label_2 Break)
            (elif (!= (Utilities|Array|FindItem (Variables|/Game/Blueprints/BP_Note.BP_Note_C|Getbeams (Utilities|Array|Get(acopy) _notes_bass _index_2)) "continue") -1)
              (Utilities|Array|Add (LocalVariables|Getlocal_continued_notes) (Utilities|Array|Get(acopy) _notes_bass _index_2)))))
        (:Completed
          (Utilities|FlowControl|Sequence
            (:then_0
              (for _array_element_2 (LocalVariables|Getlocal_continued_notes)
                (Variables|/Game/Blueprints/BP_Note.BP_Note_C|Setcontinued _array_element_2 true)
                (Default|UpdateContinueBeamMeshes _array_element_2 (Transformation|GetWorldLocation (Variables|/Game/Blueprints/BP_Note.BP_Note_C|Getbeam_attach_point start_note)) (Transformation|GetWorldLocation (Variables|/Game/Blueprints/BP_Note.BP_Note_C|Getbeam_attach_point (Utilities|Array|Get(acopy) _notes_bass _index_2))) (Variables|/Game/Blueprints/BP_Note.BP_Note_C|Getflipped start_note))))
            (:then_1
              (return (Utilities|Array|Get(acopy) _notes_bass _index_2) (LocalVariables|Getlocal_valid_return)))))))))