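; Beam actor that renders a segmented beam of spline meshes from its location to EndLocation.
; BeginPlay fills BeamSpline with evenly interpolated points, then DrawSpline adds one spline mesh per segment.
; When the actor moves, Tick re-fits those meshes to the spline's current world points without recomputing the curve toward EndLocation.
; An unused DrawDebugLine helper can trace the spline in red.
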(event EventBeginPlay
  (bind _curve_points (CallFunction|CreateCurveArray (Transformation|GetActorLocation self) (Variables|Default|Getend_location) 2))
  (Spline|SetSplinePoints (Variables|Default|Getbeam_spline) _curve_points "World" true)
  (CallFunction|DrawSpline)
  (Variables|Default|Setold_location (Transformation|GetActorLocation self)))

(event EventTick
  (params (DeltaSeconds :type Float%20%28single-precision%29))
  (bind _self self)
  (bind _returnvalue (Transformation|GetActorLocation _self))
  (if (Math|Vector|NotEqual(Vector) (Variables|Default|Getold_location) _returnvalue 0.0001)
    (CallFunction|UpdateSpline)
    (Variables|Default|Setold_location _returnvalue)))

(fn ConstructionScript)

(fn CreateCurveArray
  (params (start_point :type Vector) (end_point :type Vector) (segments :type Integer))
  (for _index (range 0 segments)
    (Utilities|Array|Add (LocalVariables|Getlocal_curve_points) (Math|Vector|Lerp(Vector) start_point end_point (/ (Math|Conversions|ToFloat(Integer) _index) (Math|Conversions|ToFloat(Integer) segments)))))
  (return (LocalVariables|Getlocal_curve_points)))

(fn DrawSpline
  (bind _beam_spline (Variables|Default|Getbeam_spline))
  (bind _returnvalue (Spline|GetNumberOfSplinePoints _beam_spline))
  (bind _returnvalue_2 (- _returnvalue 2))
  (for _index (range 0 _returnvalue_2)
    (if (== _index 0)
      (bind _returnvalue_3 (AddComponent|AddSplineMeshComponent true))
      (SplineMesh|SetStartandEnd _returnvalue_3 (.Location (Spline|GetLocationandTangentatSplinePoint _beam_spline _index "World")) (.Tangent (Spline|GetLocationandTangentatSplinePoint _beam_spline _index "World")) (.Location (Spline|GetLocationandTangentatSplinePoint _beam_spline (+ _index 1) "World")) (.Tangent (Spline|GetLocationandTangentatSplinePoint _beam_spline (+ _index 1) "World")) true :!class /Script/Engine.SplineMeshComponent)
      (Utilities|Array|Add (Variables|Default|Getspline_mesh_components) _returnvalue_3)
      (elif (== _index _returnvalue_2)
        (bind _returnvalue_4 (AddComponent|AddSplineMeshComponent true))
        (SplineMesh|SetStartandEnd _returnvalue_4 (.Location (Spline|GetLocationandTangentatSplinePoint _beam_spline _index "World")) (.Tangent (Spline|GetLocationandTangentatSplinePoint _beam_spline _index "World")) (.Location (Spline|GetLocationandTangentatSplinePoint _beam_spline (+ _index 1) "World")) (.Tangent (Spline|GetLocationandTangentatSplinePoint _beam_spline (+ _index 1) "World")) true :!class /Script/Engine.SplineMeshComponent)
        (Utilities|Array|Add (Variables|Default|Getspline_mesh_components) _returnvalue_4)
        (else
          (bind _returnvalue_5 (AddComponent|AddSplineMeshComponent true))
          (SplineMesh|SetStartandEnd _returnvalue_5 (.Location (Spline|GetLocationandTangentatSplinePoint _beam_spline _index "World")) (.Tangent (Spline|GetLocationandTangentatSplinePoint _beam_spline _index "World")) (.Location (Spline|GetLocationandTangentatSplinePoint _beam_spline (+ _index 1) "World")) (.Tangent (Spline|GetLocationandTangentatSplinePoint _beam_spline (+ _index 1) "World")) true :!class /Script/Engine.SplineMeshComponent)
          (Utilities|Array|Add (Variables|Default|Getspline_mesh_components) _returnvalue_5))))))

(fn UpdateSpline
  (bind _beam_spline (Variables|Default|Getbeam_spline))
  (for (_array_element _array_index) (Variables|Default|Getspline_mesh_components)
    (SplineMesh|SetStartandEnd _array_element (.Location (Spline|GetLocationandTangentatSplinePoint _beam_spline _array_index "World")) (.Tangent (Spline|GetLocationandTangentatSplinePoint _beam_spline _array_index "World")) (.Location (Spline|GetLocationandTangentatSplinePoint _beam_spline (+ _array_index 1) "World")) (.Tangent (Spline|GetLocationandTangentatSplinePoint _beam_spline (+ _array_index 1) "World")) true :!class /Script/Engine.SplineMeshComponent)))

(fn DrawDebugLine
  (bind _beam_spline (Variables|Default|Getbeam_spline))
  (for _index (range 0 (- (Spline|GetNumberOfSplinePoints _beam_spline) 2))
    (Rendering|Debug|DrawDebugLine (.Location (Spline|GetLocationandTangentatSplinePoint _beam_spline _index "World")) (.Location (Spline|GetLocationandTangentatSplinePoint _beam_spline (+ _index 1) "World")) "(R=0.683333,G=0.000000,B=0.000000,A=1.000000)" 2.0 2.0)))