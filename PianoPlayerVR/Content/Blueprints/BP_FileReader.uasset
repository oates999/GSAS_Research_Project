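; BP_FileReader imports a hardcoded Game of Thrones piano song on BeginPlay from treble and bass text files.
; It splits delimited text into measures, merging notes, rests and chords into offset-sorted note structs, with alternate constructors for offsets flagged as bad time.
; After debug-printing each measure, it fills "NA" time signatures from the preceding measure and passes both clef arrays to a spawned BP_MeasureSpawner.
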(event EventBeginPlay
  (bind _self self)
  (bind _returnvalue (Transformation|GetActorTransform _self))
  (Utilities|FlowControl|Sequence
    (:then_0
      ;[1 1 1] Treble Clef Import
      (for _array_element (Utilities|String|ParseIntoArray (.RightS (Utilities|String|Split (.SaveTextA (Class|ReadTxtFile|LoadTxt "Content/Assets/SongTxtFiles/GameOfThronesEasy__Piano_G.txt")) "[#]")) "[MEASURE]")
        (bind _notes (CallFunction|GetNotesfromStrings (.notes_ (Utilities|GetDatafromMeasure _array_element)) (.chords (Utilities|GetDatafromMeasure _array_element)) (.rests_ (Utilities|GetDatafromMeasure _array_element))))
        (Helper|PrintMeasureStruct (Utilities|Struct|MakeMeasure (.number (Utilities|GetDatafromMeasure _array_element)) (.time (Utilities|GetDatafromMeasure _array_element)) _notes) 2.0)
        (Utilities|Array|Add (Variables|Default|Getmeasures_treble) (Utilities|Struct|MakeMeasure (.number (Utilities|GetDatafromMeasure _array_element)) (.time (Utilities|GetDatafromMeasure _array_element)) _notes))))
    (:then_1
      ;[1 1 1] Bass Clef Import
      (for _array_element_2 (Utilities|String|ParseIntoArray (.RightS (Utilities|String|Split (.SaveTextA (Class|ReadTxtFile|LoadTxt "Content/Assets/SongTxtFiles/GameOfThronesEasy__Piano_F.txt")) "[#]")) "[MEASURE]")
        (bind _notes_2 (CallFunction|GetNotesfromStrings (.notes_ (Utilities|GetDatafromMeasure _array_element_2)) (.chords (Utilities|GetDatafromMeasure _array_element_2)) (.rests_ (Utilities|GetDatafromMeasure _array_element_2))))
        (Helper|PrintMeasureStruct (Utilities|Struct|MakeMeasure (.number (Utilities|GetDatafromMeasure _array_element_2)) (.time (Utilities|GetDatafromMeasure _array_element_2)) _notes_2) 2.0)
        (Utilities|Array|Add (Variables|Default|Getmeasures_bass) (Utilities|Struct|MakeMeasure (.number (Utilities|GetDatafromMeasure _array_element_2)) (.time (Utilities|GetDatafromMeasure _array_element_2)) _notes_2))))
    (:then_2
      (Helper|CleanOutput)
      (Game|SpawnActorfromClass "/Game/Blueprints/BP_MeasureSpawner.BP_MeasureSpawner_C" (Math|Transform|MakeTransform (.location _returnvalue) (.rotation _returnvalue) (* (.scale _returnvalue) (Variables|Default|Getscale_multiplier))) "Undefined" 0 (Variables|Default|Getmeasures_treble) (Variables|Default|Getmeasures_bass) 0))))

(fn ConstructionScript)

(fn PrintNoteStruct
  (params (note :type Note%20Structure) (duration :type Float%20%28single-precision%29))
  (bind (_offset _is_note _is_chord _is_rest _name _pitches _chord_symbol _chord_type _type _quarter_length _dots _articulations _expressions _beams _ties) (Utilities|Struct|BreakNote note))
  (bind _returnvalue (Utilities|String|ToString(Float) _quarter_length))
  (bind _returnvalue_2 (Utilities|String|ToString(Integer) _dots))
  (bind _returnvalue_3 (Utilities|String|ToString(Float) _offset))
  (if _is_note
    (Development|PrintString (Utilities|String|Append "[NOTE]  " _returnvalue_3 ", " _name ", " _type ", " _returnvalue ", " _returnvalue_2 ", " _articulations ", " (Utilities|String|ToString(Integer) 0) ", " _beams ", " _ties) true true "(R=0.000000,G=0.660000,B=1.000000,A=1.000000)" duration)
    (else
      (Development|PrintString (Utilities|String|Append "[REST]  " _returnvalue_3 ", " _type ", " _returnvalue ", " _returnvalue_2) true true "(R=0.000000,G=0.660000,B=1.000000,A=1.000000)" duration))))

(fn GetNotesfromStrings
  (params (notes_string :type String) (chords_string :type String) (rests_string :type String))
  (bind _returnvalue (Utilities|String|ParseIntoArray chords_string "[CHORD]"))
  (bind _returnvalue_2 (Utilities|String|ParseIntoArray rests_string "[REST]"))
  (bind _returnvalue_3 (Utilities|String|ParseIntoArray notes_string "[NOTE]"))
  (Utilities|FlowControl|Sequence
    (:then_0
      ;[1 1 1 1 12] Add Notes to Array
      (if (Utilities|Enum|NotEqual(Enum) (Utilities|Array|Get(acopy) _returnvalue_3) "none")
        (for _array_element _returnvalue_3
          (if (.bad_time (Utilities|ConstructNotefromNote _array_element))
            (Utilities|Array|Add (LocalVariables|Getlocal_notes) (Utilities|ConstructNotefromNoteAlt _array_element))
            (else
              (Utilities|Array|Add (LocalVariables|Getlocal_notes) (.note_struct (Utilities|ConstructNotefromNote _array_element))))))))
    (:then_1
      ;[1 1 1 1 12] Add Rests to Array
      (if (Utilities|Enum|NotEqual(Enum) (Utilities|Array|Get(acopy) _returnvalue_2) "none")
        (for _array_element_2 _returnvalue_2
          (if (.bad_time (Utilities|ConstructNotefromRest _array_element_2))
            (Utilities|Array|Add (LocalVariables|Getlocal_notes) (Utilities|ConstructNotefromRestAlt _array_element_2))
            (else
              (Utilities|Array|Add (LocalVariables|Getlocal_notes) (.note_struct (Utilities|ConstructNotefromRest _array_element_2))))))))
    (:then_2
      ;[1 1 1 1 12] Add Chords to Array
      (if (Utilities|Enum|NotEqual(Enum) (Utilities|Array|Get(acopy) _returnvalue) "none")
        (for _array_element_3 _returnvalue
          (if (.bad_time (Utilities|ConstructNotefromChord _array_element_3))
            (Utilities|Array|Add (LocalVariables|Getlocal_notes) (Utilities|ConstructNotefromChordAlt _array_element_3))
            (else
              (Utilities|Array|Add (LocalVariables|Getlocal_notes) (.note_struct (Utilities|ConstructNotefromChord _array_element_3))))))))
    (:then_3
      ;[1 1 1 1 12] Sort by Offset
      (bind _sorted_notes (Helper|SortNoteArray (LocalVariables|Getlocal_notes)))
      (return _sorted_notes))))

(fn SortNoteArray
  (params (notes :type Array%20of%20Note%20Structures))
  (bind _local_offsets (LocalVariables|Getlocal_offsets))
  (bind _output_get (LocalVariables|Setlocal_notes notes))
  (for _array_element _output_get
    (Utilities|Array|Add (LocalVariables|Getlocal_offsets) (.offset (Utilities|Struct|BreakNote _array_element))))
  (while (> (Utilities|Array|Length _local_offsets) 0)
    (LocalVariables|Setcurrent_min (.IndexOfMinValue (Math|Float|MinOfFloatArray _local_offsets)))
    (Utilities|Array|Add (LocalVariables|Getlocal_notes_sorted) (Utilities|Array|Get(acopy) (LocalVariables|Getlocal_notes) (LocalVariables|Getcurrent_min)))
    (Utilities|Array|RemoveIndex (LocalVariables|Getlocal_offsets) (LocalVariables|Getcurrent_min))
    (Utilities|Array|RemoveIndex (LocalVariables|Getlocal_notes) (LocalVariables|Getcurrent_min)))
  (return (LocalVariables|Getlocal_notes_sorted)))

(fn PrintMeasureStruct
  (params (measure :type Measure%20Structure) (duration :type Float%20%28single-precision%29))
  (bind (_number _time_signature _notes) (Utilities|Struct|BreakMeasure measure))
  (Development|PrintString (Utilities|String|Append "Measure Number " (Utilities|String|ToString(Integer) _number) " (" _time_signature "):") true true "(R=0.000000,G=0.660000,B=1.000000,A=1.000000)" duration)
  (for _array_element _notes
    (Helper|PrintNoteStruct _array_element duration)))

(fn CleanOutput
  (bind _measures_treble (Variables|Default|Getmeasures_treble))
  (bind _measures_bass (Variables|Default|Getmeasures_bass))
  (Utilities|FlowControl|Sequence
    (:then_0
      ;[1 1 1] Fix Missing TimeSignatures
      (for (_array_element _array_index) _measures_treble
        (if (Utilities|Enum|Equal(Enum) (.time_signature (Utilities|Struct|BreakMeasure _array_element)) "NA")
          (Utilities|Array|SetArrayElem _measures_treble _array_index (Utilities|Struct|MakeMeasure (.number (Utilities|Struct|BreakMeasure _array_element)) (.time_signature (Utilities|Struct|BreakMeasure (Utilities|Array|Get(acopy) _measures_treble (- _array_index 1)))) (.notes (Utilities|Struct|BreakMeasure _array_element))))))
      (for (_array_element_2 _array_index_2) _measures_bass
        (if (Utilities|Enum|Equal(Enum) (.time_signature (Utilities|Struct|BreakMeasure _array_element_2)) "NA")
          (Utilities|Array|SetArrayElem _measures_bass _array_index_2 (Utilities|Struct|MakeMeasure (.number (Utilities|Struct|BreakMeasure _array_element_2)) (.time_signature (Utilities|Struct|BreakMeasure (Utilities|Array|Get(acopy) _measures_bass (- _array_index_2 1)))) (.notes (Utilities|Struct|BreakMeasure _array_element_2)))))))))