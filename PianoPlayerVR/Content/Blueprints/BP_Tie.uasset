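; BP_Tie is an actor that draws a curved tie of spline meshes from its location to EndLocation.
; On BeginPlay, CreateCurveArray samples a Z parabola, signed by CurveDirection and scaled by distance, parameterized on X alone.
; DrawSpline adds a mesh component per segment, with separate branches for first, middle and last.
; Tick re-reads the spline into those meshes but never recomputes the curve.
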(event EventBeginPlay
  (bind _curve_points (CallFunction|CreateCurveArray (Transformation|GetActorLocation self) (Variables|Default|Getend_location) 6 (Variables|Default|Getcurve_direction) 0.065))
  (Spline|SetSplinePoints (Variables|Default|Gettie_spline) _curve_points "World" true)
  (CallFunction|DrawSpline))

(event EventTick
  (params (DeltaSeconds :type Float%20%28single-precision%29))
  (CallFunction|UpdateSpline))

(fn ConstructionScript)

(fn CreateCurveArray
  (params (start_point :type Vector) (end_point :type Vector) (segments :type Integer) (direction :type Integer) (curve_multiplier :type Float%20%28single-precision%29))
  (bind _returnvalue (- end_point start_point))
  (bind _x (Math|Vector|BreakVector end_point))
  (bind _x_2 (Math|Vector|BreakVector start_point))
  (bind _returnvalue_2 (* _returnvalue 0.5))
  (bind _returnvalue_3 (+ _returnvalue_2 start_point))
  (for _index (range 0 segments)
    (Utilities|Array|Add (LocalVariables|Getlocal_curve_points) (Math|Vector|MakeVector (.x (+ (* _returnvalue (/ (Math|Conversions|ToFloat(Integer) _index) (Math|Conversions|ToFloat(Integer) segments))) start_point)) (.y (+ (* _returnvalue (/ (Math|Conversions|ToFloat(Integer) _index) (Math|Conversions|ToFloat(Integer) segments))) start_point)) (+ (.z (+ (* _returnvalue (/ (Math|Conversions|ToFloat(Integer) _index) (Math|Conversions|ToFloat(Integer) segments))) start_point)) (* (Class|KismetMathLibrary|SignOfInteger direction) (* (* (- (.x (+ (* _returnvalue (/ (Math|Conversions|ToFloat(Integer) _index) (Math|Conversions|ToFloat(Integer) segments))) start_point)) _x_2) (- (.x (+ (* _returnvalue (/ (Math|Conversions|ToFloat(Integer) _index) (Math|Conversions|ToFloat(Integer) segments))) start_point)) _x)) (/ (* (Math|Vector|VectorLength _returnvalue) curve_multiplier) (* (- (.x _returnvalue_3) _x_2) (- (.x _returnvalue_3) _x)))))))))
  (return (LocalVariables|Getlocal_curve_points)))

(fn DrawSpline
  (bind _tie_spline (Variables|Default|Gettie_spline))
  (bind _returnvalue (Spline|GetNumberOfSplinePoints _tie_spline))
  (bind _returnvalue_2 (- _returnvalue 2))
  (for _index (range 0 _returnvalue_2)
    (if (== _index 0)
      (bind _returnvalue_3 (AddComponent|AddSplineMeshComponent true))
      (SplineMesh|SetStartandEnd _returnvalue_3 (.Location (Spline|GetLocationandTangentatSplinePoint _tie_spline _index "World")) (.Tangent (Spline|GetLocationandTangentatSplinePoint _tie_spline _index "World")) (.Location (Spline|GetLocationandTangentatSplinePoint _tie_spline (+ _index 1) "World")) (.Tangent (Spline|GetLocationandTangentatSplinePoint _tie_spline (+ _index 1) "World")) true :!class /Script/Engine.SplineMeshComponent)
      (Utilities|Array|Add (Variables|Default|Getspline_mesh_components) _returnvalue_3)
      (elif (== _index _returnvalue_2)
        (bind _returnvalue_4 (AddComponent|AddSplineMeshComponent true))
        (SplineMesh|SetStartandEnd _returnvalue_4 (.Location (Spline|GetLocationandTangentatSplinePoint _tie_spline _index "World")) (.Tangent (Spline|GetLocationandTangentatSplinePoint _tie_spline _index "World")) (.Location (Spline|GetLocationandTangentatSplinePoint _tie_spline (+ _index 1) "World")) (.Tangent (Spline|GetLocationandTangentatSplinePoint _tie_spline (+ _index 1) "World")) true :!class /Script/Engine.SplineMeshComponent)
        (Utilities|Array|Add (Variables|Default|Getspline_mesh_components) _returnvalue_4)
        (else
          (bind _returnvalue_5 (AddComponent|AddSplineMeshComponent true))
          (SplineMesh|SetStartandEnd _returnvalue_5 (.Location (Spline|GetLocationandTangentatSplinePoint _tie_spline _index "World")) (.Tangent (Spline|GetLocationandTangentatSplinePoint _tie_spline _index "World")) (.Location (Spline|GetLocationandTangentatSplinePoint _tie_spline (+ _index 1) "World")) (.Tangent (Spline|GetLocationandTangentatSplinePoint _tie_spline (+ _index 1) "World")) true :!class /Script/Engine.SplineMeshComponent)
          (Utilities|Array|Add (Variables|Default|Getspline_mesh_components) _returnvalue_5))))))

(fn UpdateSpline
  (bind _tie_spline (Variables|Default|Gettie_spline))
  (for (_array_element _array_index) (Variables|Default|Getspline_mesh_components)
    (SplineMesh|SetStartandEnd _array_element (.Location (Spline|GetLocationandTangentatSplinePoint _tie_spline _array_index "World")) (.Tangent (Spline|GetLocationandTangentatSplinePoint _tie_spline _array_index "World")) (.Location (Spline|GetLocationandTangentatSplinePoint _tie_spline (+ _array_index 1) "World")) (.Tangent (Spline|GetLocationandTangentatSplinePoint _tie_spline (+ _array_index 1) "World")) true :!class /Script/Engine.SplineMeshComponent)))